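; AI-controlled pawn that runs the BT_AdvancedAI behavior tree on BeginPlay and limits how long it fires continuously.
; Tick accumulates firing time while Firing is set and resets it otherwise.
; A one-second looping timer, re-armed by its own FireTooLong event, calls StopFire once that time exceeds two seconds.
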(event Custom|FireTooLong
  (Utilities|Time|SetTimerbyEvent (delegate Custom|FireTooLong) 1.0 true)
  (if (> (Variables|Default|GetHowLongFiring) 2.0)
    (Class|SCharacter|StopFire)))

(event EventBeginPlay
  (bind _self self)
  (bind _returnvalue (AI|GetAIController _self))
  (Utilities|IsValid _returnvalue
    (:Is%20Valid
      (AI|RunBehaviorTree _returnvalue "/Game/AdvancedAI/BT_AdvancedAI.BT_AdvancedAI")
      (CallFunction|FireTooLong))))

(event EventTick
  (params (DeltaSeconds :type Float%20%28single-precision%29))
  (if (Variables|Default|GetFiring)
    (Variables|Default|SetHowLongFiring (+ (Variables|Default|GetHowLongFiring) DeltaSeconds))
    (else
      (Variables|Default|SetHowLongFiring 0.0))))

(fn ConstructionScript)