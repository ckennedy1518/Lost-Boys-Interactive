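; Mob spawner Blueprint for a tower defense game, handling the UI side of waves and tower damage.
; DisplayWaveStart shows a WaveBegin widget with an optional save prompt, then removes it after a delay and clears FirstWave.
; UItoViewport briefly flashes the in-game UI unless the camera pawn or its own flag reports it visible.
; BeginPlay adds the QuitGame widget after a short delay, and BlueprintMTGCalled forwards to MTGCalled.
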(event EventDisplayWaveStart
  (params (ShowSave :type Boolean))
  (bind _returnvalue (UserInterface|CreateWidget "/Game/TowerDefense/Blueprints/UI/WaveBegin.WaveBegin_C" (Game|GetPlayerController 0) ShowSave))
  (UserInterface|Viewport|AddtoViewport _returnvalue 0)
  (Utilities|FlowControl|Delay 1e+01)
  (Utilities|IsValid _returnvalue
    (:Is%20Valid
      (Widget|RemovefromParent _returnvalue)
      (Variables|Default|SetFirstWave false))))

(event EventUItoViewport
  (bind _astower_defense_camera_pawn (Utilities|Casting|CastToTowerDefenseCameraPawn (Game|Player|GetPlayerPawn 0)))
  (if (not (or (Variables|/Game/TowerDefense/Blueprints/TowerDefenseCameraPawn.TowerDefenseCameraPawn_C|GetUIVisible _astower_defense_camera_pawn) (Variables|Default|GetUIVisibleDamageTower)))
    (bind _returnvalue (UserInterface|CreateWidget "/Game/TowerDefense/Blueprints/UI/UserInterfaceInGame.UserInterfaceInGame_C"))
    (bind _output_get (Variables|Default|SetUIWidget _returnvalue))
    (UserInterface|Viewport|AddtoViewport _output_get 0)
    (Variables|Default|SetUIVisibleDamageTower true)
    (Utilities|FlowControl|Delay 2.0)
    (Widget|RemovefromParent (Variables|Default|GetUIWidget))
    (Variables|Default|SetUIVisibleDamageTower false)))

(event EventBeginPlay
  (Utilities|FlowControl|Delay 0.5)
  (bind _returnvalue (UserInterface|CreateWidget "/Game/TowerDefense/Blueprints/UI/QuitGame.QuitGame_C"))
  (UserInterface|Viewport|AddtoViewport _returnvalue 0))

(fn ConstructionScript)

(fn BlueprintMTGCalled
  (Class|CPPMobSpawner|MTGCalled))