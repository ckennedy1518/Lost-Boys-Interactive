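; BP_OpalItem is an opal inventory item Blueprint that prepares a slate brush from M_OpalImage on BeginPlay.
; UpdateUI finds the first BP_InventoryManager and calls GetUsefulItems on it, without using the result.
; GetPositionInInventory records the first opal's index, then runs an empty loop from there to the list's end.
; Unconnected logic would flag FirstPersonCharacter's first useful slot and set its image to the opal brush.
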(event Custom|GetPositionInInventory
  (params (UsefulItems :type Array%20of%20PG%20Inventory%20Item%20Class%20References))
  (bind (_array_element _array_index) (Utilities|Array|ForEachLoopwithBreak UsefulItems :!label _label) ; Loop gets position of first opal
    (:LoopBody
      (if (== _array_element "BP_OpalItem_C")
        (Variables|Default|SetIndexOfOpal _array_index)
        (goto _label Break)))
    (:Completed
      (for _index (range (Variables|Default|GetIndexOfOpal) (- (Utilities|Array|Length UsefulItems) 1))
        _))))

(event EventBeginPlay
  (Variables|Default|SetOpalSlateBrush (Utilities|Struct|MakeSlateBrush "(X=250.000000,Y=135.000000)" "(Left=0.000000,Top=0.000000,Right=0.000000,Bottom=0.000000)" "(SpecifiedColor=(R=1.000000,G=1.000000,B=1.000000,A=1.000000),ColorUseRule=UseColor_Specified)" "/Game/Blueprints/Items/ItemImages/M_OpalImage.M_OpalImage" "Image" "NoTile" "NoMirror")))

(event EventUpdateUI
  (bind _outactors (Actor|GetAllActorsOfClass "/Game/Blueprints/BP_InventoryManager.BP_InventoryManager_C"))
  (Utilities|IsValid (Utilities|Array|Get(acopy) _outactors)
    (:Is%20Valid
      (Class|PGInventoryManager|GetUsefulItems (Utilities|Array|Get(acopy) _outactors)) ; Already in order
    )))

(fn ConstructionScript)