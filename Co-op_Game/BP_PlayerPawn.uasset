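; Player pawn for the co-op game that manages the local player's HUD widgets.
; On BeginPlay, a locally controlled pawn creates crosshair, health and level info widgets, passing itself to level info.
; A fixed delay lets the weapon exist before the reload widget receives CurrentWeapon.
; RemoveWidgetsfromViewport clears all four only if the reload widget is valid, otherwise it prints a debug message.
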(event EventRemoveWidgetsfromViewport
  (bind _reloadwidget (Variables|Default|GetReloadWidget))
  (Utilities|IsValid _reloadwidget
    (:Is%20Valid
      (Widget|RemovefromParent _reloadwidget)
      (Widget|RemovefromParent (Variables|Default|GetScoreWidget))
      (Widget|RemovefromParent (Variables|Default|GetHealthWidget))
      (Widget|RemovefromParent (Variables|Default|GetCrosshairWidget)))
    (:Is%20Not%20Valid
      (Development|PrintString "Reload widget is invalid" true true "(R=0.000000,G=0.660000,B=1.000000,A=1.000000)" 2e+02))))

(event EventBeginPlay
  (if (Pawn|IsLocallyControlled)
    (bind _returnvalue (UserInterface|CreateWidget "/Game/WeaponEffects/UI/WBP_Crosshair.WBP_Crosshair_C"))
    (bind _output_get (Variables|Default|SetCrosshairWidget _returnvalue))
    (UserInterface|Viewport|AddtoViewport _output_get 0)
    (bind _returnvalue_2 (UserInterface|CreateWidget "/Game/UI/WBP_HealthIndicator.WBP_HealthIndicator_C"))
    (bind _output_get_2 (Variables|Default|SetHealthWidget _returnvalue_2))
    (UserInterface|Viewport|AddtoViewport _output_get_2 0)
    (bind _returnvalue_3 (UserInterface|CreateWidget "/Game/UI/WBP_LevelInfo.WBP_LevelInfo_C" 0 self))
    (bind _output_get_3 (Variables|Default|SetScoreWidget _returnvalue_3))
    (UserInterface|Viewport|AddtoViewport _output_get_3 0)
    (Utilities|FlowControl|Delay 2.0) ; Make sure we have weapon
    (bind _returnvalue_4 (UserInterface|CreateWidget "/Game/WeaponEffects/UI/WBP_Reload.WBP_Reload_C" 0 (Variables|Default|GetCurrentWeapon)))
    (bind _output_get_4 (Variables|Default|SetReloadWidget _returnvalue_4))
    (UserInterface|Viewport|AddtoViewport _output_get_4 0)))

(fn ConstructionScript)