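; BP_QuartzItem is a quartz item for the maze project that shows itself in the player's useful-item HUD slots.
; UpdateUI finds the inventory manager and uses its useful-item count to pick one of five slots on the FirstPersonCharacter.
; It sets that slot's flag and applies the quartz brush to its image, with debug prints for tracing and failure cases.
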(event EventUpdateUI
  (bind _returnvalue (Game|GetPlayerCharacter 0))
  (Development|PrintString "Updating quartz UI")
  (bind _outactors (Actor|GetAllActorsOfClass "/Game/Blueprints/BP_InventoryManager.BP_InventoryManager_C"))
  (Utilities|IsValid (Utilities|Array|Get(acopy) _outactors)
    (:Is%20Valid
      (bind _returnvalue_2 (Class|PGInventoryManager|GetUsefulItems (Utilities|Array|Get(acopy) _outactors)))
      (Development|PrintString (Utilities|String|Append "Length of collectable items: " (Utilities|String|ToString(Integer) (Utilities|Array|Length _returnvalue_2))))
      (switch int (Utilities|Array|Length _returnvalue_2)
        (:0
          (Development|PrintString "Useful item length is 0? Either item being added after or GetUsefulItems() not working"))
        (:1
          (bind _asfirst_person_character (Utilities|Casting|CastToFirstPersonCharacter _returnvalue))
          (Variables|/Game/FirstPersonCPP/Blueprints/FirstPersonCharacter.FirstPersonCharacter_C|SetUseful1 _asfirst_person_character true)
          (Class|Image|SetBrush (Variables|/Game/FirstPersonCPP/Blueprints/FirstPersonCharacter.FirstPersonCharacter_C|GetUsefulSlot1Image _asfirst_person_character) (Variables|Default|GetQuartzSlateBrush))
          (Development|PrintString "Setting brush 1"))
        (:2
          (bind _asfirst_person_character_2 (Utilities|Casting|CastToFirstPersonCharacter _returnvalue))
          (Variables|/Game/FirstPersonCPP/Blueprints/FirstPersonCharacter.FirstPersonCharacter_C|SetUseful2 _asfirst_person_character_2 true)
          (Class|Image|SetBrush (Variables|/Game/FirstPersonCPP/Blueprints/FirstPersonCharacter.FirstPersonCharacter_C|GetUsefulSlot2Image _asfirst_person_character_2) (Variables|Default|GetQuartzSlateBrush)))
        (:3
          (bind _asfirst_person_character_3 (Utilities|Casting|CastToFirstPersonCharacter _returnvalue))
          (Variables|/Game/FirstPersonCPP/Blueprints/FirstPersonCharacter.FirstPersonCharacter_C|SetUseful3 _asfirst_person_character_3 true)
          (Class|Image|SetBrush (Variables|/Game/FirstPersonCPP/Blueprints/FirstPersonCharacter.FirstPersonCharacter_C|GetUsefulSlot3Image _asfirst_person_character_3) (Variables|Default|GetQuartzSlateBrush)))
        (:4
          (bind _asfirst_person_character_4 (Utilities|Casting|CastToFirstPersonCharacter _returnvalue))
          (Variables|/Game/FirstPersonCPP/Blueprints/FirstPersonCharacter.FirstPersonCharacter_C|SetUseful4 _asfirst_person_character_4 true)
          (Class|Image|SetBrush (Variables|/Game/FirstPersonCPP/Blueprints/FirstPersonCharacter.FirstPersonCharacter_C|GetUsefulSlot4Image _asfirst_person_character_4) (Variables|Default|GetQuartzSlateBrush)))
        (:5
          (bind _asfirst_person_character_5 (Utilities|Casting|CastToFirstPersonCharacter _returnvalue))
          (Variables|/Game/FirstPersonCPP/Blueprints/FirstPersonCharacter.FirstPersonCharacter_C|SetUseful5 _asfirst_person_character_5 true)
          (Class|Image|SetBrush (Variables|/Game/FirstPersonCPP/Blueprints/FirstPersonCharacter.FirstPersonCharacter_C|GetUsefulSlot5Image _asfirst_person_character_5) (Variables|Default|GetQuartzSlateBrush)))))
    (:Is%20Not%20Valid
      (Development|PrintString "Inventory manager is invalid?" true true "(R=0.000000,G=0.660000,B=1.000000,A=1.000000)" 2e+02))))

(fn ConstructionScript)