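; Monster character in the procedural maze that runs the BT_Monster behavior tree and hands it the single player and itself through blackboard keys.
; Tick either eases the monster to face the player until roughly aligned, or runs a timed field reset.
; The reset interpolates monster and player back to the field center and player start, turning monster and control rotation toward each other.
; LookAtPlayer applies one small turn step and returns whether yaw still differs.
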(event Custom|SetCenterLoc
  (params (Position :type Vector))
  (Variables|Default|SetCenterLoc Position))

(event EventBeginPlay
  (bind _self self)
  (bind _returnvalue (AI|GetBlackboard _self))
  (AI|RunBehaviorTree (AI|GetAIController self) "/Game/Monster/AI/BT_Monster.BT_Monster")
  (bind _asproc_gen_maze_character (Utilities|Casting|CastToProcGenMazeCharacter (Game|GetPlayerCharacter 0)))
  (AI|Components|Blackboard|SetValueasObject _returnvalue (Utilities|Name|MakeLiteralName "PlayerCharacter") _asproc_gen_maze_character) ; We only need to set this once,\nit isn't like the Coop game where\nthere are multiple players
  (AI|Components|Blackboard|SetValueasObject _returnvalue (Utilities|Name|MakeLiteralName "SelfActor") self))

(event EventTick
  (params (DeltaSeconds :type Float%20%28single-precision%29))
  (bind _returnvalue (Transformation|GetActorRotation))
  (bind _centerloc (Variables|Default|GetCenterLoc))
  (Variables|Default|SetDelta DeltaSeconds)
  (if (Variables|Default|GetRotateTowardsPlayer)
    (bind _asproc_gen_maze_character (Utilities|Casting|CastToProcGenMazeCharacter (Game|GetPlayerCharacter 0)))
    (Transformation|SetActorRotation (Math|Interpolation|RInterpTo _returnvalue (Math|Rotator|FindLookatRotation (Transformation|GetActorLocation) (Transformation|GetActorLocation _asproc_gen_maze_character)) (Variables|Default|GetDelta) 5.0))
    (if (Math|Rotator|Equal(Rotator) _returnvalue (Math|Rotator|FindLookatRotation (Transformation|GetActorLocation) (Transformation|GetActorLocation _asproc_gen_maze_character)) 5.0)
      (Variables|Default|SetRotateTowardsPlayer false))
    (elif (Variables|Default|GetResetField)
      (Transformation|SetActorLocation (Math|Interpolation|VInterpTo (Transformation|GetActorLocation) (Variables|Default|GetCenterLoc) (Variables|Default|GetDelta) 3.0) false false)
      (bind _asproc_gen_maze_character_2 (Utilities|Casting|CastToProcGenMazeCharacter (Game|GetPlayerCharacter 0)))
      (Variables|Default|SetPlayerStartInField (Class|ProcGenMazeCharacter|GetPlayerMonsterStartLocation _asproc_gen_maze_character_2))
      (Transformation|SetActorLocation _asproc_gen_maze_character_2 (Math|Interpolation|VInterpTo (Transformation|GetActorLocation _asproc_gen_maze_character_2) (Variables|Default|GetPlayerStartInField) (Variables|Default|GetDelta) 3.0) false false)
      (Transformation|SetActorRotation (Math|Interpolation|RInterpTo (Transformation|GetActorRotation _asproc_gen_maze_character_2) (Math|Rotator|FindLookatRotation _centerloc (Variables|Default|GetPlayerStartInField)) (Variables|Default|GetDelta) 0.0))
      (bind _asbp_player_controller (Utilities|Casting|CastToBP_PlayerController (Pawn|GetController _asproc_gen_maze_character_2)))
      (Pawn|SetControlRotation _asbp_player_controller (Math|Interpolation|RInterpTo (Transformation|GetActorRotation) (Math|Rotator|FindLookatRotation (Variables|Default|GetPlayerStartInField) _centerloc) (Variables|Default|GetDelta) 0.0))
      (bind _output_get (Variables|Default|SetTickingLength (+ (Variables|Default|GetTickingLength) (Variables|Default|GetDelta))))
      (if (> _output_get 5.0)
        (Variables|Default|SetResetField false)
        (Variables|Default|SetTickingLength 0.0)))))

(fn ConstructionScript)

(fn LookatPlayer
  (bind _asproc_gen_maze_character (Utilities|Casting|CastToProcGenMazeCharacter (Game|GetPlayerCharacter 0)))
  (Transformation|SetActorRotation (Math|Interpolation|RInterpTo (Transformation|GetActorRotation _asproc_gen_maze_character) (Math|Rotator|MakeRotator 0.0 0.0 (.Yaw (Math|Rotator|BreakRotator (Math|Rotator|FindLookatRotation (Transformation|GetActorLocation) (Transformation|GetActorLocation _asproc_gen_maze_character))))) 0.05 1.0))
  (return (!= (.Yaw (Math|Rotator|BreakRotator (Transformation|GetActorRotation _asproc_gen_maze_character))) (.Yaw (Math|Rotator|BreakRotator (Math|Rotator|FindLookatRotation (Transformation|GetActorLocation) (Transformation|GetActorLocation _asproc_gen_maze_character)))))))