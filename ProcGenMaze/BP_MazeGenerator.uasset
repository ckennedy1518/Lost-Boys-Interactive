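; BP_MazeGenerator handles monster spawning and navigation bounds for the procedural maze; no maze-building logic appears here.
; SpawnMonster spawns a BP_Monster, raises it, sets its center location and spawns a scaled RecastNavMesh actor nearby.
; DespawnMonster destroys the stored monster.
; UpdateNavMesh moves and scales the first existing NavMeshBoundsVolume, then notifies the navigation system, reusing one volume for runtime navmesh updates.
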(event EventSpawnMonster
  (params (SpawnLoc :type Vector :default "0, 0, 0"))
  (bind _returnvalue (Game|SpawnActorfromClass "/Game/Monster/BP_Monster.BP_Monster_C" (Math|Conversions|ToTransform(Vector) SpawnLoc) "AdjustIfPossibleButAlwaysSpawn" 0 0))
  (bind _output_get (Variables|Default|SetMonsterInGame _returnvalue))
  (Transformation|SetActorLocation _output_get (+ (Transformation|GetActorLocation _output_get) "0, 0,50.000000") false false)
  (Default|SetCenterLoc (Variables|Default|GetMonsterInGame) (+ (Transformation|GetActorLocation _output_get) "0, 0,50.000000"))
  (Game|SpawnActorfromClass "/Script/NavigationSystem.RecastNavMesh" (Math|Transform|MakeTransform (+ (Transformation|GetActorLocation _output_get) "0, 0,50.000000") "0, 0, 0" "50.000000,50.000000,3.000000") "Undefined" 0 0))

(event EventDespawnMonster
  (bind _monsteringame (Variables|Default|GetMonsterInGame))
  (Utilities|IsValid _monsteringame
    (:Is%20Valid
      (Actor|DestroyActor _monsteringame))))

(event EventUpdateNavMesh
  (params (Location :type Vector :default "0, 0, 0") (Scale :type Vector :default "0, 0, 0"))
  (bind _outactors (Actor|GetAllActorsOfClass "/Script/NavigationSystem.NavMeshBoundsVolume"))
  (Utilities|IsValid (Utilities|Array|Get(acopy) _outactors)
    (:Is%20Valid
      (Transformation|SetActorLocation (Utilities|Array|Get(acopy) _outactors) Location false false)
      (Transformation|SetActorScale3D (Utilities|Array|Get(acopy) _outactors) Scale)
      (Class|NavigationSystemV1|OnNavigationBoundsUpdated (Class|NavigationSystemV1|GetNavigationSystem) (Utilities|Array|Get(acopy) _outactors)))))

(fn ConstructionScript)