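; BP_RubberDuckItem is a rubber duck collectable that updates the player's collectable slots in the UI.
; UpdateUI finds the first BP_InventoryManager and switches on its collectable item count, from one to five.
; Each case sets the matching Collectable flag on FirstPersonCharacter and applies the duck brush to a slot image.
; The third case writes to slot 2's image, and debug prints report the count or an invalid manager.
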(event EventUpdateUI
  (bind _returnvalue (Game|GetPlayerCharacter 0))
  (bind _outactors (Actor|GetAllActorsOfClass "/Game/Blueprints/BP_InventoryManager.BP_InventoryManager_C"))
  (Utilities|IsValid (Utilities|Array|Get(acopy) _outactors)
    (:Is%20Valid
      (bind _returnvalue_2 (Class|PGInventoryManager|GetCollectableItems (Utilities|Array|Get(acopy) _outactors)))
      (Development|PrintString (Utilities|String|Append "Length of collectable items: " (Utilities|String|ToString(Integer) (Utilities|Array|Length _returnvalue_2))))
      (switch int (Utilities|Array|Length _returnvalue_2)
        (:1
          (bind _asfirst_person_character (Utilities|Casting|CastToFirstPersonCharacter _returnvalue))
          (Variables|/Game/FirstPersonCPP/Blueprints/FirstPersonCharacter.FirstPersonCharacter_C|SetCollectable1 _asfirst_person_character true)
          (Class|Image|SetBrush (Variables|/Game/FirstPersonCPP/Blueprints/FirstPersonCharacter.FirstPersonCharacter_C|GetCollectableSlot1Image _asfirst_person_character) (Variables|Default|GetRubberDuckSlateBrush)))
        (:2
          (bind _asfirst_person_character_2 (Utilities|Casting|CastToFirstPersonCharacter _returnvalue))
          (Variables|/Game/FirstPersonCPP/Blueprints/FirstPersonCharacter.FirstPersonCharacter_C|SetCollectable2 _asfirst_person_character_2 true)
          (Class|Image|SetBrush (Variables|/Game/FirstPersonCPP/Blueprints/FirstPersonCharacter.FirstPersonCharacter_C|GetCollectableSlot2Image _asfirst_person_character_2) (Variables|Default|GetRubberDuckSlateBrush)))
        (:3
          (bind _asfirst_person_character_3 (Utilities|Casting|CastToFirstPersonCharacter _returnvalue))
          (Variables|/Game/FirstPersonCPP/Blueprints/FirstPersonCharacter.FirstPersonCharacter_C|SetCollectable3 _asfirst_person_character_3 true)
          (Class|Image|SetBrush (Variables|/Game/FirstPersonCPP/Blueprints/FirstPersonCharacter.FirstPersonCharacter_C|GetCollectableSlot2Image _asfirst_person_character_3) (Variables|Default|GetRubberDuckSlateBrush)))
        (:4
          (bind _asfirst_person_character_4 (Utilities|Casting|CastToFirstPersonCharacter _returnvalue))
          (Variables|/Game/FirstPersonCPP/Blueprints/FirstPersonCharacter.FirstPersonCharacter_C|SetCollectable4 _asfirst_person_character_4 true)
          (Class|Image|SetBrush (Variables|/Game/FirstPersonCPP/Blueprints/FirstPersonCharacter.FirstPersonCharacter_C|GetCollectableSlot4Image _asfirst_person_character_4) (Variables|Default|GetRubberDuckSlateBrush)))
        (:5
          (bind _asfirst_person_character_5 (Utilities|Casting|CastToFirstPersonCharacter _returnvalue))
          (Variables|/Game/FirstPersonCPP/Blueprints/FirstPersonCharacter.FirstPersonCharacter_C|SetCollectable5 _asfirst_person_character_5 true)
          (Class|Image|SetBrush (Variables|/Game/FirstPersonCPP/Blueprints/FirstPersonCharacter.FirstPersonCharacter_C|GetCollectableSlot5Image _asfirst_person_character_5) (Variables|Default|GetRubberDuckSlateBrush)))))
    (:Is%20Not%20Valid
      (Development|PrintString "Invalid?" true true "(R=0.000000,G=0.660000,B=1.000000,A=1.000000)" 2e+02))))

(fn ConstructionScript)